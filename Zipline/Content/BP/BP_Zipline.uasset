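; Zipline actor that strings a cable between two end points and offers them to overlapping actors as a ride in either direction.
; The construction script and BeginPlay both move the cable to the start top and attach its far end to the end top.
; Each end's collider sends SetZiplineMessage on overlap with that end as start and the opposite as destination, and disables it on exit.
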(event OnComponentBeginOverlap(StartCollider)
  (params (OverlappedComponent :type Primitive%20Component%20Object%20Reference) (OtherActor :type Actor%20Object%20Reference) (OtherComp :type Primitive%20Component%20Object%20Reference) (OtherBodyIndex :type Integer) (bFromSweep :type Boolean) (SweepResult :type Hit%20Result%20Structure%20%28by%20ref%29))
  (Class|BPIZipline|SetZipline(Message) OtherActor true (Transformation|GetWorldLocation (Variables|Default|Getstart%20top)) (Transformation|GetWorldLocation (Variables|Default|GetEnd%20Top))))

(event OnComponentEndOverlap(StartCollider)
  (params (OverlappedComponent :type Primitive%20Component%20Object%20Reference) (OtherActor :type Actor%20Object%20Reference) (OtherComp :type Primitive%20Component%20Object%20Reference) (OtherBodyIndex :type Integer))
  (Class|BPIZipline|SetZipline(Message) OtherActor false "0, 0, 0" "0, 0, 0"))

(event OnComponentBeginOverlap(EndCollider)
  (params (OverlappedComponent :type Primitive%20Component%20Object%20Reference) (OtherActor :type Actor%20Object%20Reference) (OtherComp :type Primitive%20Component%20Object%20Reference) (OtherBodyIndex :type Integer) (bFromSweep :type Boolean) (SweepResult :type Hit%20Result%20Structure%20%28by%20ref%29))
  (Class|BPIZipline|SetZipline(Message) OtherActor true (Transformation|GetWorldLocation (Variables|Default|GetEnd%20Top)) (Transformation|GetWorldLocation (Variables|Default|Getstart%20top))))

(event OnComponentEndOverlap(EndCollider)
  (params (OverlappedComponent :type Primitive%20Component%20Object%20Reference) (OtherActor :type Actor%20Object%20Reference) (OtherComp :type Primitive%20Component%20Object%20Reference) (OtherBodyIndex :type Integer))
  (Class|BPIZipline|SetZipline(Message) OtherActor false "0, 0, 0" "0, 0, 0"))

(event EventBeginPlay
  (Utilities|NewMacro))

(event Collision|EventActorBeginOverlap
  (params (OtherActor :type Actor%20Object%20Reference)))

(event EventTick
  (params (DeltaSeconds :type Float%20%28single-precision%29)))

(fn ConstructionScript
  (|InitCable))

(fn NewFunction)